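; BP_GrassArea is a box volume that tells herd AI actors whether they are standing on grass.
; Box overlap begin and end events pass the other actor to UpdateGrassArea, which writes the on-grass bool into that BP_Herd_AI's blackboard.
; Shortly after BeginPlay, a delayed sweep of the box's overlapping actors also flags any herd AI that starts inside it.
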(event OnComponentBeginOverlap(Box)
  (params (OverlappedComponent :type Primitive%20Component%20Object%20Reference) (OtherActor :type Actor%20Object%20Reference) (OtherComp :type Primitive%20Component%20Object%20Reference) (OtherBodyIndex :type Integer) (bFromSweep :type Boolean) (SweepResult :type Hit%20Result%20Structure%20%28by%20ref%29))
  (CallFunction|UpdateGrassArea true OtherActor))

(event OnComponentEndOverlap(Box)
  (params (OverlappedComponent :type Primitive%20Component%20Object%20Reference) (OtherActor :type Actor%20Object%20Reference) (OtherComp :type Primitive%20Component%20Object%20Reference) (OtherBodyIndex :type Integer))
  (CallFunction|UpdateGrassArea false OtherActor))

(event EventBeginPlay
  (Utilities|FlowControl|Delay 0.2)
  (for _array_element (Collision|GetOverlappingActors (Variables|Default|GetBox) 0 :!class /Script/Engine.PrimitiveComponent)
    (CallFunction|UpdateGrassArea true _array_element)))

(event Collision|EventActorBeginOverlap
  (params (OtherActor :type Actor%20Object%20Reference)))

(event EventTick
  (params (DeltaSeconds :type Float%20%28single-precision%29)))

(fn ConstructionScript)

(fn UpdateGrassArea
  (params (IsGrass :type Boolean) (OverlapActor :type Actor%20Object%20Reference))
  (bind _asbp_herd_ai (Utilities|Casting|CastToBP_Herd_AI OverlapActor))
  (AI|Components|Blackboard|SetValueasBool (AI|GetBlackboard _asbp_herd_ai) (LocalVariables|GetKey_OnGrass) IsGrass))