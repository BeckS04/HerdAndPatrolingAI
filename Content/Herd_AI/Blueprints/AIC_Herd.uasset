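; AI controller for a single herd deer, running the herd behavior tree on possession and reacting when it sees the player.
; A successful sight of a visible Human-tagged character sets the deer's state to startled and writes the spotted human and state to the Blackboard.
; A restartable timer then blocks further sight reactions until it expires, and the behavior tree can call the same event to reset it.
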(event OnTargetPerceptionUpdated(AIPerception)
  (params (Actor :type Actor%20Object%20Reference) (Stimulus :type AI%20Stimulus%20Structure))
  ;[1 1 1] Conditions before sight can be sensed, must be sight of the player (Human Tag), successfully  sensed and the timer must not be set)
  (bind _returnvalue (Class|AIPerceptionSystem|GetSenseClassforStimulus Stimulus))
  (if (and (== _returnvalue "/Script/AIModule.AISense_Sight") (Actor|ActorHasTag Actor "Human"))
    (bind _cansense (CallFunction|CanReactSense Actor Stimulus))
    ;[1 1 1] sets the single deer into the startled state
    (if _cansense
      (bind _asbp_herd_ai (Utilities|Casting|CastToBP_Herd_AI (Variables|Default|GetPossessed%20Pawn)))
      (Default|UpdateState _asbp_herd_ai "NewEnumerator6")
      (AI|Components|Blackboard|SetValueasObject (AI|GetBlackboard _asbp_herd_ai) (Variables|Default|GetSpottedHuman) Actor)
      (bind _output_get (Variables|Default|SetState "NewEnumerator6"))
      (AI|Components|Blackboard|SetValueasEnum (AI|GetBlackboard _asbp_herd_ai) (Variables|Default|GetKey_State) _output_get)
      ;;[1 1 1] Makes sure the sight sense can only be called again after timer runs out, event is called from behaviour tree to reset the previous timer
      (Utilities|Time|InvalidateTimerHandle (Variables|Default|GetResetSenseTimer))
      (bind _returnvalue_2 (Utilities|Time|SetTimerbyEvent (delegate Custom|ResetSense) (Variables|Default|GetStartledTimer)))
      (Variables|Default|SetResetSenseTimer _returnvalue_2)
      (Variables|Default|SetHasJustSeen true))))

(event Custom|DeerNewTimer
  ;[1 1 1] sets the single deer into the startled state
  ;;[1 1 1] Makes sure the sight sense can only be called again after timer runs out, event is called from behaviour tree to reset the previous timer
  (Utilities|Time|InvalidateTimerHandle (Variables|Default|GetResetSenseTimer))
  (bind _returnvalue (Utilities|Time|SetTimerbyEvent (delegate Custom|ResetSense) (Variables|Default|GetStartledTimer)))
  (Variables|Default|SetResetSenseTimer _returnvalue)
  (Variables|Default|SetHasJustSeen true))

(event Custom|ResetSense
  ;[1 1 1] sets the single deer into the startled state
  ;;[1 1 1] Makes sure the sight sense can only be called again after timer runs out, event is called from behaviour tree to reset the previous timer
  (Variables|Default|SetHasJustSeen false))

(event EventBeginPlay)

(event EventTick
  (params (DeltaSeconds :type Float%20%28single-precision%29)))

(event EventPossess
  (params (PossessedPawn :type Pawn%20Object%20Reference))
  (Variables|Default|SetPossessed%20Pawn PossessedPawn)
  (AI|RunBehaviorTree "/Game/Herd_AI/Behaviour/BT_Herd.BT_Herd"))

(fn ConstructionScript)

(fn CanReactSense
  (params (SensedActor :type Actor%20Object%20Reference) (SenseUsed :type AI%20Stimulus%20Structure))
  ;[1 1 1] Gives back true as long as the sens was succesfull, the target is not hidden and it hasnt just seen something until the timer ran out or the deer reached its destination
  (bind _asthird_person_character (Utilities|Casting|CastToThirdPersonCharacter SensedActor)
    (:then
      (return (Math|Boolean|ANDBoolean (not (Variables|/Game/Player_Level_BP/Blueprints/ThirdPersonCharacter.ThirdPersonCharacter_C|GetIsHidden _asthird_person_character)) (Utilities|Struct|BreakAIStimulus SenseUsed) (not (Variables|Default|GetHasJustSeen)))))
    (:CastFailed
      (return false))))