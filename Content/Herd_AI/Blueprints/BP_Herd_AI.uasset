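; BP_Herd_AI is a herd animal character that tracks food, water and a behavior state for its AI.
; On BeginPlay it randomizes both needs to desynchronize the herd, starts Roaming and launches a one-second looping timer.
; Each tick of that timer copies the leader's state into its Blackboard, drains and publishes water, and drains food only while Fleeing.
; UpdateState stores the new state and sets the matching walk speed.
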(event Custom|SyncStates
  (bind _self self)
  (bind _key_currentwater (Variables|Default|GetKey_CurrentWater))
  (bind _returnvalue (AI|GetAIController _self))
  (bind _returnvalue_2 (AI|GetBlackboard _returnvalue))
  ;[1 1 1] this does the initial update, also starts a looping timer that updates stats such as water food and where the leader is every second. For food synch while roaming was used, because the stat is only important while roaming and does not interrupt any other stat
  (bind _asbp_herd_ai (Utilities|Casting|CastToBP_Herd_AI (AI|Components|Blackboard|GetValueasObject (AI|GetBlackboard (AI|GetAIController self)) (Variables|Default|GetKey_Leader)))
    (:then
      (AI|Components|Blackboard|SetValueasEnum (AI|GetBlackboard (AI|GetAIController self)) (Variables|Default|GetKey_LeaderState) (Class|BlackboardComponent|GetValueasEnum (AI|GetBlackboard (AI|GetAIController _asbp_herd_ai)) (Variables|Default|GetKey_State))))
    (:CastFailed
      _))
  (if (Utilities|Enum|Equal(Enum) (Variables|Default|GetState) "NewEnumerator2")
    (bind _output_get (Variables|Default|SetWater (- (Variables|Default|GetWater) 3.0)))
    (AI|Components|Blackboard|SetValueasFloat _returnvalue_2 _key_currentwater _output_get)
    (Variables|Default|SetFood (- (Variables|Default|GetFood) 1.5))
    (else
      (bind _output_get_2 (Variables|Default|SetWater (- (Variables|Default|GetWater) 1.0)))
      (AI|Components|Blackboard|SetValueasFloat _returnvalue_2 _key_currentwater _output_get_2))))

(event EventBeginPlay
  ;[1 1 1] this does the initial update, also starts a looping timer that updates stats such as water food and where the leader is every second. For food synch while roaming was used, because the stat is only important while roaming and does not interrupt any other stat
  ;;[1 1 1] Random value for water and foot so it’s not snychronous
  (Variables|Default|SetFood (Math|Random|RandomFloatinRange 1e+02 4e+02))
  (Variables|Default|SetWater (Math|Random|RandomFloatinRange 8e+01 1.6e+02))
  (CallFunction|UpdateState "NewEnumerator1")
  (Utilities|Time|SetTimerbyEvent (delegate Custom|SyncStates) 1.0 true))

(fn ConstructionScript)

(fn UpdateSpeed
  (params (New%20Walk%20Speed :type Float%20%28single-precision%29))
  ;[1 1 1] function name says it all
  (Variables|/Script/Engine.CharacterMovementComponent|SetMaxWalkSpeed (Variables|Character|GetCharacterMovement) New%20Walk%20Speed))

(fn UpdateState
  (params (NewState :type E_AnimalState%20Enum :default "NewEnumerator0"))
  ;[1 1 1] updates the state and the speed for state
  (bind _output_get (Variables|Default|SetState NewState))
  (switch Utilities|FlowControl|Switch|SwitchonE_AnimalState _output_get
    (:NewEnumerator0
      (CallFunction|UpdateSpeed 0.0 :!label _label))
    (:NewEnumerator1
      (CallFunction|UpdateSpeed 1e+02 :!label _label_2))
    (:NewEnumerator2
      (CallFunction|UpdateSpeed 7e+02 :!label _label_3))
    (:NewEnumerator3
      (goto _label_2))
    (:NewEnumerator4
      (goto _label))
    (:NewEnumerator6
      (goto _label_3))
    (:NewEnumerator7
      (goto _label))
    (:NewEnumerator8
      (CallFunction|UpdateSpeed 3.5e+02 :!label _label_4))
    (:NewEnumerator9
      (goto _label_4))))