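; BP_ShieldRegen is an area actor that triggers shield regeneration for BP_Enemy_AI enemies inside its sphere.
; On sphere overlap by an exact BP_Enemy_AI, it shows the Shield component and calls ShieldRegenEntered on that enemy.
; On end overlap it hides Shield and calls ShieldRegenLeft, without counting occupants, so one enemy leaving hides it even if others remain.
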(event OnComponentBeginOverlap(Sphere)
  (params (OverlappedComponent :type Primitive%20Component%20Object%20Reference) (OtherActor :type Actor%20Object%20Reference) (OtherComp :type Primitive%20Component%20Object%20Reference) (OtherBodyIndex :type Integer) (bFromSweep :type Boolean) (SweepResult :type Hit%20Result%20Structure%20%28by%20ref%29))
  ;[1 1 1] When overlapped with actor of class enemy ai start his shield regen event, when leaving the overlap call the event to stop shield regeneration.
  (if (== (Utilities|GetClass OtherActor) "/Game/Enemy_AI/Blueprints/BP_Enemy_AI.BP_Enemy_AI_C")
    (Rendering|SetVisibility (Variables|Default|GetShield) true false)
    (bind _asbp_enemy_ai (Utilities|Casting|CastToBP_Enemy_AI OtherActor))
    (Default|ShieldRegenEntered _asbp_enemy_ai)))

(event OnComponentEndOverlap(Sphere)
  (params (OverlappedComponent :type Primitive%20Component%20Object%20Reference) (OtherActor :type Actor%20Object%20Reference) (OtherComp :type Primitive%20Component%20Object%20Reference) (OtherBodyIndex :type Integer))
  ;[1 1 1] When overlapped with actor of class enemy ai start his shield regen event, when leaving the overlap call the event to stop shield regeneration.
  (if (== (Utilities|GetClass OtherActor) "/Game/Enemy_AI/Blueprints/BP_Enemy_AI.BP_Enemy_AI_C")
    (Rendering|SetVisibility (Variables|Default|GetShield) false false)
    (bind _asbp_enemy_ai (Utilities|Casting|CastToBP_Enemy_AI OtherActor))
    (Default|ShieldRegenLeft _asbp_enemy_ai)))

(event EventBeginPlay)

(event Collision|EventActorBeginOverlap
  (params (OtherActor :type Actor%20Object%20Reference)))

(event EventTick
  (params (DeltaSeconds :type Float%20%28single-precision%29)))

(fn ConstructionScript)