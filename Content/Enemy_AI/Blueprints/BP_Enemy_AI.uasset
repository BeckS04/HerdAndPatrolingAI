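; Enemy AI character with a regenerating shield that absorbs damage before health, mirroring both values to its AI Blackboard.
; Damage spawns Niagara effects when the shield breaks or the enemy dies and is destroyed.
; Regen-field enter and leave events start and stop a looping timer that refills and restores the shield.
; State changes set walk speed, while attack and weapon actions play animations and flag them on the Blackboard.
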(event OnComponentHit(Shield)
  (params (HitComponent :type Primitive%20Component%20Object%20Reference) (OtherActor :type Actor%20Object%20Reference) (OtherComp :type Primitive%20Component%20Object%20Reference) (NormalImpulse :type Vector :default "0, 0, 0") (Hit :type Hit%20Result%20Structure%20%28by%20ref%29))
  ;[1 1 1] just spawns particle, for the shield hit effect at the hit location when hit since only projectiles can hit the shield. Damage event happens from the projectiles blueprint.
  (Niagara|SpawnSystematLocation "/Game/VFX_And_Materials/VFX/NS_ShieldHit.NS_ShieldHit" (.ImpactPoint (Collision|BreakHitResult Hit)) "0, 0,0.000000"))

(event Custom|ShieldRegenLeft
  ;[1 1 1] Leaves regen field stops regen per s
  (Utilities|Time|ClearandInvalidateTimerbyHandle (Variables|Default|GetTimerShieldRegen)))

(event Custom|RegenShield
  (bind _blackboardused (Variables|Default|GetBlackboardUsed))
  (bind _key_shieldhp (Variables|Default|GetKey_ShieldHP))
  ;[1 1 1] Entered regen shield, starts shield regen per s as long as enemy doesn't leave the field
  (if (< (Variables|Default|GetShieldHp) (Variables|Default|GetMaxHpShield))
    (if (< (+ (Variables|Default|GetShieldHp) 15.0) (Variables|Default|GetMaxHpShield))
      (bind _output_get (Variables|Default|SetShieldHp (+ (Variables|Default|GetShieldHp) 15.0)))
      (AI|Components|Blackboard|SetValueasFloat _blackboardused _key_shieldhp _output_get)
      (else
        (bind _output_get_2 (Variables|Default|SetShieldHp (Variables|Default|GetMaxHpShield)))
        (AI|Components|Blackboard|SetValueasFloat _blackboardused _key_shieldhp _output_get_2)))
    (Components|StaticMesh|SetStaticMesh (Variables|Default|GetShield) "/Engine/BasicShapes/Sphere.Sphere")))

(event Custom|ShieldRegenEntered
  ;[1 1 1] Entered regen shield, starts shield regen per s as long as enemy doesn't leave the field
  (bind _returnvalue (Utilities|Time|SetTimerbyEvent (delegate Custom|RegenShield) 1.0 true))
  (Variables|Default|SetTimerShieldRegen _returnvalue))

(event EventBeginPlay
  (Utilities|FlowControl|Delay 0.2)
  (Variables|Default|SetBlackboardUsed (AI|GetBlackboard (AI|GetAIController self)))
  (AI|Components|Blackboard|SetValueasFloat (Variables|Default|GetBlackboardUsed) (Variables|Default|GetKey_ShieldHP) (Variables|Default|GetShieldHp))
  (AI|Components|Blackboard|SetValueasFloat (Variables|Default|GetBlackboardUsed) (Variables|Default|GetKey_CharacterHP) (Variables|Default|GetCharacterHp)))

(event EventTick
  (params (DeltaSeconds :type Float%20%28single-precision%29)))

(fn ConstructionScript)

(fn UpdateSpeed
  (params (NewSpeed :type Float%20%28single-precision%29))
  (Variables|/Script/Engine.CharacterMovementComponent|SetMaxWalkSpeed (Variables|Character|GetCharacterMovement) NewSpeed))

(fn StartAttack
  (Components|Animation|PlayAnimation (Variables|Character|GetMesh) "/Game/Mannequin/Animations/Stable_Sword_Outward_Slash_Anim_mixamo_com.Stable_Sword_Outward_Slash_Anim_mixamo_com" false)
  (bind _output_get (Variables|Default|SetAnimationPlaying true))
  (AI|Components|Blackboard|SetValueasBool (AI|GetBlackboard (AI|GetAIController self)) (Variables|Default|GetKey_AnimationPlaying) _output_get))

(fn RecieveDamage
  (params (Amount :type Float%20%28single-precision%29))
  (bind _shield (Variables|Default|GetShield))
  ;[1 1 1] Damage Calculation, when shield is destroyed spawn particle system for destroyed shield. When hp reach 0 or lower, destroy the actor and spawn the particle system for when an actor gets destroyed
  (LocalVariables|SetDamageAmount Amount)
  (if (> (Variables|Default|GetShieldHp) 0.0)
    (bind _output_get (Variables|Default|SetShieldHp (- (Variables|Default|GetShieldHp) (LocalVariables|GetDamageAmount))))
    (if (not (<= _output_get 0.0))
      _
      (else
        (Niagara|SpawnSystematLocation "/Game/VFX_And_Materials/VFX/NS_ShieldDestroyed.NS_ShieldDestroyed" (Transformation|GetWorldLocation _shield))
        (Components|StaticMesh|SetStaticMesh _shield 0)))
    (AI|Components|Blackboard|SetValueasFloat (Variables|Default|GetBlackboardUsed) (Variables|Default|GetKey_ShieldHP) _output_get)
    (else
      (bind _output_get_2 (Variables|Default|SetCharacterHp (- (Variables|Default|GetCharacterHp) (LocalVariables|GetDamageAmount))))
      (if (> _output_get_2 0.0)
        (AI|Components|Blackboard|SetValueasFloat (Variables|Default|GetBlackboardUsed) (Variables|Default|GetKey_CharacterHP) _output_get_2)
        (else
          (Niagara|SpawnSystematLocation "/Game/VFX_And_Materials/VFX/NS_PlayerDestroyed.NS_PlayerDestroyed" (Transformation|GetActorLocation))
          (Actor|DestroyActor))))))

(fn UpdateState
  (params (NewParam :type E_EnemyStates%20Enum :default "NewEnumerator0"))
  (bind _output_get (Variables|Default|SetState NewParam))
  (switch Utilities|FlowControl|Switch|SwitchonE_EnemyStates _output_get
    (:NewEnumerator6
      (CallFunction|UpdateSpeed 0.0 :!label _label))
    (:NewEnumerator0
      (CallFunction|UpdateSpeed 2.5e+02))
    (:NewEnumerator1
      (CallFunction|UpdateSpeed 4.5e+02 :!label _label_2))
    (:NewEnumerator3
      (CallFunction|UpdateSpeed 1.2e+02))
    (:NewEnumerator4
      (goto _label))
    (:NewEnumerator7
      (goto _label_2))
    (:NewEnumerator8
      (goto _label_2))
    (:NewEnumerator9
      (goto _label))
    (:NewEnumerator10
      (goto _label_2))))

(fn DrawWeapon
  ;[1 1 1] Draw/undraw weapon, just plays animation and sets the bool to true. Animations has notify that makes sure to inform the blackboard when animation has ended.
  (Variables|Default|SetWeaponEquipped true)
  (Components|Animation|PlayAnimation (Variables|Character|GetMesh) "/Game/Mannequin/Animations/Equip_Over_Shoulder.Equip_Over_Shoulder" false)
  (bind _output_get (Variables|Default|SetAnimationPlaying true))
  (AI|Components|Blackboard|SetValueasBool (AI|GetBlackboard (AI|GetAIController self)) (Variables|Default|GetKey_AnimationPlaying) _output_get))

(fn UnDrawWeapon
  ;[1 1 1] Draw/undraw weapon, just plays animation and sets the bool to true. Animations has notify that makes sure to inform the blackboard when animation has ended.
  (Variables|Default|SetWeaponEquipped true)
  (Components|Animation|PlayAnimation (Variables|Character|GetMesh) "/Game/Mannequin/Animations/UnEquip_Over_Shoulder.UnEquip_Over_Shoulder" false)
  (bind _output_get (Variables|Default|SetAnimationPlaying true))
  (AI|Components|Blackboard|SetValueasBool (AI|GetBlackboard (AI|GetAIController self)) (Variables|Default|GetKey_AnimationPlaying) _output_get))