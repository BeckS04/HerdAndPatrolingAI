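; Spline-based patrol path actor that supplies looping waypoints to enemy AI and places shield regen areas along the route.
; Shortly after BeginPlay, it registers itself in the Blackboard of each BP_Enemy_AI sharing its first actor tag.
; It then spawns a BP_ShieldRegen at every spline point.
; Helper functions return a point's world location and the next index, wrapping around in either direction.
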(event EventBeginPlay
  ;[1 1 1] Find related enemy, init variables, spawn shieldRegen areas at every patrol path along the spline of this actor
  (Utilities|FlowControl|Delay 0.2)
  (bind _outactors (Actor|GetAllActorsOfClass "/Game/Enemy_AI/Blueprints/BP_Enemy_AI.BP_Enemy_AI_C"))
  (for _array_element _outactors
    (if (Actor|ActorHasTag _array_element (Utilities|Array|Get(acopy) (Variables|Actor|GetTags)))
      (AI|Components|Blackboard|SetValueasObject (AI|GetBlackboard _array_element) (Variables|Default|GetKey_PatrolPath) self)))
  (bind _result (Math|Integer|DecrementInt (Spline|GetNumberOfSplinePoints (Variables|Default|GetSpline)))
    (:%20%20
      (bind _output_get (Variables|Default|SetPointsIndexCount _result))
      (for _index (range 0 _output_get)
        (bind _newparam (CallFunction|GetPatrolPointLocation _index))
        (Game|SpawnActorfromClass "/Game/Enemy_AI/Blueprints/BP_ShieldRegen.BP_ShieldRegen_C" (Math|Conversions|ToTransform(Vector) _newparam) "Undefined" 0 0)))))

(fn ConstructionScript)

(fn GetPatrolPointLocation
  (params (IndexPoint :type Integer))
  (return (Spline|GetLocationatSplinePoint (Variables|Default|GetSpline) IndexPoint "World")))

(fn GetNextPatrolPoint
  (params (MovingBackwards :type Boolean) (CurrentPoint :type Integer))
  (LocalVariables|SetLoc_CurrentPoint CurrentPoint)
  (if MovingBackwards
    (if (== (LocalVariables|GetLoc_CurrentPoint) 0)
      (return (Variables|Default|GetPointsIndexCount))
      (else
        (return (- (LocalVariables|GetLoc_CurrentPoint) 1))))
    (elif (> (+ CurrentPoint 1) (Variables|Default|GetPointsIndexCount))
      (return 0)
      (else
        (return (+ (LocalVariables|GetLoc_CurrentPoint) 1))))))