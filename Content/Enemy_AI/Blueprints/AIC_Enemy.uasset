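; AI controller for enemies that runs BT_Enemy on possess and turns perception stimuli into blackboard state, ignoring them while an animation plays.
; Sounds startle enemies that are not attacking or chasing into investigating the noise location, throttled by a one-second timer.
; Seeing a Player-tagged actor sets it as target with line of sight.
; Losing sight starts a timer that clears both on expiry unless the player is seen again.
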(event OnTargetPerceptionUpdated(AIPerception)
  (params (Actor :type Actor%20Object%20Reference) (Stimulus :type AI%20Stimulus%20Structure))
  (bind _blackboard (Variables|Default|GetBlackboard))
  ;[1 1 1] Logic for reaction to sight and hearing
  ;;[1 1 1] Can only spot when animation ( attacking / weapon drawing )  is not playing
  (if (not (ScalableFloat|GetValueasBool (Variables|Default|GetBlackboard) (Variables|Default|GetKey_AnimationIsPlaying)))
    (Variables|Default|SetSpottedActor Actor)
    (bind _returnvalue (Class|AIPerceptionSystem|GetSenseClassforStimulus Stimulus))
    (if (and (== _returnvalue "/Script/AIModule.AISense_Hearing") (not (Variables|Default|GetjustHeardSound)))
      (CallFunction|SensHearing Actor Stimulus)
      ;;[1 1 1] Timer is needed so the enemy isnt stuck when the player is constantly shooting
      (Utilities|Time|SetTimerbyEvent (delegate Custom|HearingSensePuffer) 1.0)
      (Variables|Default|SetjustHeardSound true)
      (else
        ;;[1 1 1] Enemy Spots the player, if he can not see the player again  until the timer LoSTimer runs out and fires the event, he loses line of sight and stops chasing
        ;;;[1 1 1] So the ai doesnt lose sight on player when sensing other ai actors
        (if (Actor|ActorHasTag Actor "Player")
          (bind _true (CallFunction|SensSeeing Actor Stimulus))
          (if _true
            (Utilities|Time|ClearandInvalidateTimerbyHandle (Variables|Default|GetLoSTimer))
            (AI|Components|Blackboard|SetValueasObject _blackboard (Variables|Default|GetKey_EnemyActor) (Variables|Default|GetSpottedActor))
            (AI|Components|Blackboard|SetValueasBool _blackboard (Variables|Default|GetKey_HasLineOfSight) true)
            (AI|Components|Blackboard|SetValueasEnum _blackboard (Variables|Default|GetKey_State) 2)
            (else
              (bind _returnvalue_2 (Utilities|Time|SetTimerbyEvent (delegate Custom|LoSTimer_Event) (Variables|Default|GetT_LineOfSight)))
              (Variables|Default|SetLoSTimer _returnvalue_2))))))))

(event Custom|LoSTimer_Event
  (bind _blackboard (Variables|Default|GetBlackboard))
  ;[1 1 1] Logic for reaction to sight and hearing
  ;;[1 1 1] Enemy Spots the player, if he can not see the player again  until the timer LoSTimer runs out and fires the event, he loses line of sight and stops chasing
  (AI|Components|Blackboard|SetValueasBool _blackboard (Variables|Default|GetKey_HasLineOfSight) false)
  (AI|Components|Blackboard|SetValueasObject _blackboard (Variables|Default|GetKey_EnemyActor) 0))

(event Custom|HearingSensePuffer
  ;[1 1 1] Logic for reaction to sight and hearing
  ;;[1 1 1] Timer is needed so the enemy isnt stuck when the player is constantly shooting
  (Variables|Default|SetjustHeardSound false))

(event EventBeginPlay)

(event EventTick
  (params (DeltaSeconds :type Float%20%28single-precision%29)))

(event EventPossess
  (params (PossessedPawn :type Pawn%20Object%20Reference))
  (AI|RunBehaviorTree "/Game/Enemy_AI/Behaviour/BT_Enemy.BT_Enemy"))

(fn ConstructionScript)

(fn SensHearing
  (params (ActorNoise :type Actor%20Object%20Reference) (Stimilus :type AI%20Stimulus%20Structure))
  (bind _statestarteled (LocalVariables|GetStateStarteled))
  (bind _blackboard (Variables|Default|GetBlackboard))
  (bind _blackboard_2 (Variables|Default|GetBlackboard))
  (bind _key_state (Variables|Default|GetKey_State))
  (bind _returnvalue (Class|BlackboardComponent|GetValueasEnum _blackboard_2 _key_state))
  (bind _returnvalue_2 (Utilities|Enum|ByteToEnumE_EnemyStates _returnvalue))
  ;[1 1 1] As long as the enemy ai is currently neither attacking nor chasing, this will set the state to starteled, which will then start the investigation state
  (if (Math|Boolean|NORBoolean (Utilities|Enum|Equal(Enum) _returnvalue_2 "NewEnumerator1") (Utilities|Enum|Equal(Enum) _returnvalue_2 "NewEnumerator4"))
    (AI|Components|Blackboard|SetValueasObject _blackboard (Variables|Default|GetKey_EnemyActor) ActorNoise)
    (AI|Components|Blackboard|SetValueasVector _blackboard (Variables|Default|GetKey_LastEnemyLocation) (Utilities|Struct|BreakAIStimulus Stimilus))
    (bind _asbp_enemy_ai (Utilities|Casting|CastToBP_Enemy_AI (Pawn|GetControlledPawn self)))
    (Default|UpdateState _asbp_enemy_ai _statestarteled)
    (AI|Components|Blackboard|SetValueasEnum (Variables|Default|GetBlackboard) (Variables|Default|GetKey_State) _statestarteled)
    (return)
    (else
      (return))))

(fn SensSeeing
  (params (ActorNoise :type Actor%20Object%20Reference) (Stimilus :type AI%20Stimulus%20Structure))
  ;[1 1 1] makes sure it was a successfull sight sense of a player
  (bind _returnvalue (Class|AIPerceptionSystem|GetSenseClassforStimulus Stimilus))
  (if (Math|Boolean|ANDBoolean (Actor|ActorHasTag ActorNoise "Player") (.bSuccessfullySensed (Utilities|Struct|BreakAIStimulus Stimilus)) (== _returnvalue "/Script/AIModule.AISense_Sight"))
    (return true)
    (else
      (return false))))